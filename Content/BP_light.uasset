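; BP_light is a blinking spotlight actor.
; The construction script sets the SpotLight's initial visibility from the IsEneble variable.
; On BeginPlay it hides and re-shows the light with two-second delays, looping back through a DoN node that caps the blink at 99 cycles.
; The blink runs regardless of IsEneble, so the light stays visible once the cycles run out.
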(event `self.ReceiveBeginPlay`
  (`/Engine/EditorBlueprintResources/StandardMacros.Do N` 99 :!label _label
    (:`Exit`
      (`SceneComponent.SetVisibility` (`self.SpotLight`) false false)
      (`KismetSystemLibrary.Delay` 2.0)
      (`SceneComponent.SetVisibility` (`self.SpotLight`) true false)
      (`KismetSystemLibrary.Delay` 2.0)
      (goto _label))))

(fn `UserConstructionScript`
  (`SceneComponent.SetVisibility` (`self.SpotLight`) (`self.isEneble`) false))